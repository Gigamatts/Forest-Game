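; BP_Lampawn is a melee enemy character that detects the player, punches, and is replaced by BP_BrokeLampawn on death.
; PawnSensing sets a Blackboard flag and custom depth on sight, which Tick clears after delays and a sight-radius distance check.
; Punch montages pair with timer-looped sphere traces meant to damage Player-tagged actors, though the hit-array loop is unwired.
; Damage plays a hit montage and launches survivors backward.
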(event OnSeePawn(PawnSensing)
  (params (Pawn :type Pawn%20Object%20Reference))
  ;[1 1 1] Viu o Player
  (Utilities|Casting|CastToThirdPersonCharacter Pawn)
  (AI|Components|Blackboard|SetValueasBool (AI|GetBlackboard (AI|GetAIController self)) (Utilities|Name|MakeLiteralName "HasSeenPlayer?") true)
  (Variables|Default|SetcanSeePlayer? true)
  (Rendering|SetRenderCustomDepth (Variables|Character|GetMesh) true))

(event Custom|AttackLampawn
  ;[1 1 1] Attack
  (if (not (Variables|Default|GetisAttacking?))
    (Variables|Default|SetisAttacking? true)
    (bind _returnvalue (Animation|PlayAnimMontage "/Game/Characters/Animations/ThirdPersonChar/Punching__1__Montage.Punching__1__Montage" 1.0 "None"))
    (Utilities|FlowControl|Delay _returnvalue)
    (Variables|Default|SetisAttacking? false)))

(event Custom|Start%20Punch%20Trace
  ;[1 1 1] Punch Trace
  (bind _returnvalue (Utilities|Time|SetTimerbyEvent (delegate Custom|Punch%20Trace%20Loop) 0.1 true))
  (Variables|Default|SetPuncTraceLoop _returnvalue))

(event Custom|Punch%20Trace%20Loop
  ;[1 1 1] Punch Trace
  (bind (_outhits _returnvalue) (Collision|MultiSphereTraceForObjects (Transformation|GetWorldLocation (Variables|Default|GetPunch%20Top%20Point)) (Transformation|GetWorldLocation (Variables|Default|GetPunch%20Bottom%20Point)) 3e+01 (Utilities|Array|MakeArray "ObjectTypeQuery3") false 0 "ForDuration" true "(R=1.000000,G=0.000000,B=0.000000,A=1.000000)" "(R=0.000000,G=1.000000,B=0.000000,A=1.000000)" 0.2))
  (if _returnvalue
    (Development|PrintString "bateu")
    (if (Actor|ActorHasTag (.HitActor (Collision|BreakHitResult (stale _array_element))) "Player")
      (Utilities|FlowControl|DoOnce false :!label _label
        (:Completed
          (Game|Damage|ApplyDamage (.HitActor (Collision|BreakHitResult (stale _array_element))) 5e+01 0 0)
          (Utilities|FlowControl|Delay 0.5)
          (goto _label Reset))))))

(event Custom|Stop%20Punch%20Trace
  ;[1 1 1] Punch Trace
  (Utilities|Time|ClearandInvalidateTimerbyHandle (Variables|Default|GetPuncTraceLoop)))

(event EventTick
  (params (DeltaSeconds :type Float%20%28single-precision%29))
  ;[1 1 1] Parou de ver
  (if (Variables|Default|GetcanSeePlayer?)
    (Utilities|FlowControl|Delay 0.5)
    (if (<= (Transformation|GetDistanceTo (Game|Player|GetPlayerPawn 0)) (Variables|/Script/AIModule.PawnSensingComponent|GetSightRadius (Variables|Default|GetPawnSensing)))
      (Utilities|FlowControl|Delay 1.0)
      (Variables|Default|SetcanSeePlayer? false)
      (AI|Components|Blackboard|SetValueasBool (AI|GetBlackboard (AI|GetAIController self)) (Utilities|Name|MakeLiteralName "HasSeenPlayer?") false)
      (Rendering|SetRenderCustomDepth (Variables|Character|GetMesh) false))))

(event Game|Damage|EventAnyDamage
  (params (Damage :type Float%20%28single-precision%29) (DamageType :type Damage%20Type%20Object%20Reference) (InstigatedBy :type Controller%20Object%20Reference) (DamageCauser :type Actor%20Object%20Reference))
  (bind _returnvalue (Math|Vector|VectorUp))
  (bind _returnvalue_2 (Transformation|GetActorForwardVector))
  (bind _charactermovement (Variables|Character|GetCharacterMovement))
  (bind _returnvalue_3 (+ _returnvalue_2 _returnvalue))
  (bind _returnvalue_4 (Math|Vector|Normalize _returnvalue_3))
  ;[1 0.06146 0.06146] Take Damege
  (bind _output_get (Variables|Default|SetHealth (- (Variables|Default|GetHealth) Damage)))
  (Animation|PlayAnimMontage "/Game/Characters/Lampawn/Animations/LampawnGetHitAnim_Montage.LampawnGetHitAnim_Montage" 1.0 "None")
  (if (<= _output_get 0.0)
    (Game|SpawnActorfromClass "/Game/NPC/Enemys/Lampiao/BrokeLampawn/BP_BrokeLampawn.BP_BrokeLampawn_C" (Transformation|GetActorTransform) "Undefined" 0 0)
    (Actor|DestroyActor)
    (else
      ;;[1 1 1] Make imune and knockback
      (if (AI|Components|NavMovement|IsFalling _charactermovement)
        (Character|StopJumping)
        (else
          (Variables|/Script/Engine.CharacterMovementComponent|SetGroundFriction _charactermovement 0.0)))
      (Variables|/Script/Engine.MovementComponent|SetVelocity _charactermovement "0, 0, 0")
      (Character|LaunchCharacter (Math|Vector|MakeVector (* (.x _returnvalue_4) -8e+02) (* (.y _returnvalue_4) -8e+02) (* (.z _returnvalue_4) 5e+02)) true true))))

(event EventBeginPlay
  (Variables|Default|SetOriginalLocationRef (Transformation|GetActorLocation)))

(fn ConstructionScript)

(fn Attack
  (bind _returnvalue (Animation|PlayAnimMontage "/Game/Characters/Lampawn/Animations/LampawnPunchAnim_Montage.LampawnPunchAnim_Montage" 1.0 "None"))
  (return _returnvalue))