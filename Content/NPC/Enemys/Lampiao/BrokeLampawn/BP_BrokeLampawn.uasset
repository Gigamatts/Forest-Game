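; Broken Lampawn enemy that reassembles its scattered pieces and then turns back into a live BP_Lampawn.
; BeginPlay records world transforms of the hands, body and head, waits, then stops their physics and lerps each back via its own timeline.
; After a short delay it disables part collision, spawns BP_Lampawn at the body's transform with a yaw offset, and destroys itself.
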(event Custom|CallEveryPart
  ;[1 1 1] Call Every Part
  (CallFunction|CallHandL)
  (CallFunction|CallHandR)
  (CallFunction|CallBodyBack)
  (CallFunction|CallHeadBack))

(event Custom|CallHandL
  (bind _handl (Variables|Default|GetHandL))
  (bind _handl_2 (Variables|Default|GetHandL))
  ;[1 1 1] Call Parts
  (Physics|SetSimulatePhysics (Variables|Default|GetHandL) false)
  (bind _x_location (Timeline|Timeline_0 PlayFromStart)
    (:Update
      (Transformation|SetWorldLocation _handl (Math|Vector|Lerp(Vector) (Transformation|GetWorldLocation _handl_2) (Variables|Default|GetHandLOriginalLocation) _x_location) false false)
      (Transformation|SetWorldRotation _handl (Math|Rotator|Lerp(Rotator) (Transformation|GetWorldRotation _handl_2) (Variables|Default|GetHandLOriginalRotation) _x_location) false false))))

(event Custom|CallHandR
  (bind _handr (Variables|Default|GetHandR))
  (bind _handr_2 (Variables|Default|GetHandR))
  ;[1 1 1] Call Parts
  (Physics|SetSimulatePhysics (Variables|Default|GetHandR) false)
  (bind _x_location (Timeline|Timeline_1 PlayFromStart)
    (:Update
      (Transformation|SetWorldLocation _handr_2 (Math|Vector|Lerp(Vector) (Transformation|GetWorldLocation _handr) (Variables|Default|GetHandROriginalLocation) _x_location) false false)
      (Transformation|SetWorldRotation _handr_2 (Math|Rotator|Lerp(Rotator) (Transformation|GetWorldRotation _handr) (Variables|Default|GetHandROriginalRotation) _x_location) false false))))

(event Custom|CallBodyBack
  (bind _body (Variables|Default|GetBody))
  (bind _body_2 (Variables|Default|GetBody))
  ;[1 1 1] Call Parts
  (Physics|SetSimulatePhysics (Variables|Default|GetBody) false)
  (bind _x_location (Timeline|Timeline_2 PlayFromStart)
    (:Update
      (Transformation|SetWorldLocation _body (Math|Vector|Lerp(Vector) (Transformation|GetWorldLocation _body_2) (Variables|Default|GetBodyOriginalLocation) _x_location) false false)
      (Transformation|SetWorldRotation _body (Math|Rotator|Lerp(Rotator) (Transformation|GetWorldRotation _body_2) (Variables|Default|GetBodyOriginalRotation) _x_location) false false))))

(event Custom|CallHeadBack
  (bind _head (Variables|Default|GetHead))
  (bind _head_2 (Variables|Default|GetHead))
  ;[1 1 1] Call Parts
  (Physics|SetSimulatePhysics (Variables|Default|GetHead) false)
  (bind _x_location (Timeline|Timeline_3 PlayFromStart)
    (:Update
      (Transformation|SetWorldLocation _head_2 (Math|Vector|Lerp(Vector) (Transformation|GetWorldLocation _head) (Variables|Default|GetHeadOriginalLocation) _x_location) false false)
      (Transformation|SetWorldRotation _head_2 (Math|Rotator|Lerp(Rotator) (Transformation|GetWorldRotation _head) (Variables|Default|GetHeadOriginalRotation) _x_location) false false))))

(event Custom|DisableColission
  ;[1 1 1] Disable Collision
  (Collision|SetCollisionEnabled (Variables|Default|GetBody) "NoCollision")
  (Collision|SetCollisionEnabled (Variables|Default|GetHandR) "NoCollision")
  (Collision|SetCollisionEnabled (Variables|Default|GetHandL) "NoCollision")
  (Collision|SetCollisionEnabled (Variables|Default|GetHead) "NoCollision"))

(event EventBeginPlay
  (bind _body (Variables|Default|GetBody))
  (bind _body_2 (Variables|Default|GetBody))
  (bind _head (Variables|Default|GetHead))
  (bind _handl (Variables|Default|GetHandL))
  (bind _handr (Variables|Default|GetHandR))
  (bind _returnvalue (Transformation|GetWorldTransform _body))
  (Variables|Default|SetHandLOriginalLocation (Transformation|GetWorldLocation _handl))
  (Variables|Default|SetHandROriginalLocation (Transformation|GetWorldLocation _handr))
  (Variables|Default|SetBodyOriginalLocation (Transformation|GetWorldLocation _body_2))
  (Variables|Default|SetHeadOriginalLocation (Transformation|GetWorldLocation _head))
  (Variables|Default|SetHandLOriginalRotation (Transformation|GetWorldRotation _handl))
  (Variables|Default|SetHandROriginalRotation (Transformation|GetWorldRotation _handr))
  (Variables|Default|SetBodyOriginalRotation (Transformation|GetWorldRotation _body_2))
  (Variables|Default|SetHeadOriginalRotation (Transformation|GetWorldRotation _head))
  (Utilities|FlowControl|Delay 5.0)
  (CallFunction|CallEveryPart)
  (Utilities|FlowControl|Delay 1.0)
  (CallFunction|DisableColission)
  (Game|SpawnActorfromClass "/Game/NPC/Enemys/Lampiao/BP_Lampawn.BP_Lampawn_C" (Math|Transform|MakeTransform (.location _returnvalue) (Math|Rotator|MakeRotator (.roll (.rotation _returnvalue)) (.pitch (.rotation _returnvalue)) (- (.yaw (.rotation _returnvalue)) -9e+01)) (.scale _returnvalue)) "Undefined" 0 0)
  (Actor|DestroyActor))

(fn ConstructionScript)