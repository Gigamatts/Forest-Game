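; Capybara NPC that offers dialog to the player, showing a bobbing indicator sprite while the player is inside its sphere.
; Tick animates the sprite with a sine and, on click or key/gamepad press, opens a DialogHandler widget with DialogRef through a DoOnce.
; Leaving the sphere plays a down montage, removes the widget and re-arms the DoOnce after the montage.
; The indicator stays hidden in MainMenuScene and is destroyed when dialog is disabled.
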(event OnComponentBeginOverlap(Sphere)
  (params (OverlappedComponent :type Primitive%20Component%20Object%20Reference) (OtherActor :type Actor%20Object%20Reference) (OtherComp :type Primitive%20Component%20Object%20Reference) (OtherBodyIndex :type Integer) (bFromSweep :type Boolean) (SweepResult :type Hit%20Result%20Structure%20%28by%20ref%29))
  (Utilities|Casting|CastToThirdPersonCharacter OtherActor)
  (Variables|Default|SetIsHide? true)
  (Variables|Default|SetisDialogable true)
  (Rendering|SetVisibility (Variables|Default|GetDialogIndicatorSprite) true false))

(event OnComponentEndOverlap(Sphere)
  (params (OverlappedComponent :type Primitive%20Component%20Object%20Reference) (OtherActor :type Actor%20Object%20Reference) (OtherComp :type Primitive%20Component%20Object%20Reference) (OtherBodyIndex :type Integer))
  (Utilities|Casting|CastToThirdPersonCharacter OtherActor)
  (Rendering|SetVisibility (Variables|Default|GetDialogIndicatorSprite) false false)
  (Utilities|FlowControl|DoOnce false :!label _label
    (:Completed
      (Variables|Default|SetIsHide? false)
      (Variables|Default|SetIsInContact false)
      (Variables|Default|SetisDialogable false)
      (bind _returnvalue (Animation|PlayAnimMontage "/Game/Characters/Capybara/Anims/capy_Down_Anim_Montage.capy_Down_Anim_Montage" 1.0 "None"))
      (Utilities|IsValid (Variables|Default|GetDialogoHandlerRef)
        (:Is%20Valid
          (Widget|RemovefromParent (Variables|Default|GetDialogoHandlerRef)))
        (:Is%20Not%20Valid
          (Variables|Default|SetDialogoHandlerRef 0)))
      (Utilities|FlowControl|Delay _returnvalue)
      (Utilities|FlowControl|Sequence
        (:then_0
          (goto _label Reset))
        (:then_1
          ;[1 1 1] Ativar o dialogo
          (Utilities|FlowControl|DoOnce false) ; enters at Reset
        )))))

(event EventTick
  (params (DeltaSeconds :type Float%20%28single-precision%29))
  (bind _returnvalue (Game|GetPlayerController 0))
  ;[1 1 1] Ativar o dialogo
  (bind _returnvalue_2 (Game|GetCurrentLevelName true))
  (if (Utilities|Enum|Equal(Enum) _returnvalue_2 "MainMenuScene")
    (Rendering|SetVisibility (Variables|Default|GetDialogIndicatorSprite) false false))
  (Transformation|AddRelativeLocation (Variables|Default|GetDialogIndicatorSprite) (Math|Vector|MakeVector 0.0 0.0 (* (* (Math|Trig|Sin(Degrees) (* (Actor|GetGameTimeSinceCreation) 1e+02)) 0.01111) 1e+02)) false false)
  (if (and (Math|Boolean|Equal(Boolean) (Variables|Default|GetisDialogable) true) (Math|Boolean|ORBoolean (Game|Player|WasInputKeyJustPressed _returnvalue "LeftMouseButton") (Game|Player|WasInputKeyJustPressed _returnvalue "Z") (Game|Player|WasInputKeyJustPressed _returnvalue "Gamepad_FaceButton_Left")))
    (Utilities|FlowControl|DoOnce false
      (:Completed
        (if (and (Variables|Default|GetDoYouWantDialog) (Rendering|IsVisible (Variables|Default|GetDialogIndicatorSprite)))
          (bind _returnvalue_3 (UserInterface|CreateWidget "/Game/UI/DialogHandler.DialogHandler_C" 0 (Variables|Default|GetdialogRef)))
          (bind _output_get (Variables|Default|SetDialogoHandlerRef _returnvalue_3))
          (UserInterface|Viewport|AddtoViewport _output_get 0))))))

(event EventBeginPlay
  (bind _dialogindicatorsprite (Variables|Default|GetDialogIndicatorSprite))
  (bind _asthird_person_character (Utilities|Casting|CastToThirdPersonCharacter (Game|GetPlayerCharacter 0)))
  (Variables|Default|SetPlayerRef _asthird_person_character)
  (Rendering|SetVisibility (Variables|Default|GetDialogIndicatorSprite) false false)
  (if (Variables|Default|GetDoYouWantDialog)
    (bind _returnvalue (Game|GetCurrentLevelName true))
    (if (Utilities|Enum|Equal(Enum) _returnvalue "MainMenuScene")
      (Rendering|SetVisibility _dialogindicatorsprite false false))
    (else
      (Components|DestroyComponent _dialogindicatorsprite))))

(fn ConstructionScript)