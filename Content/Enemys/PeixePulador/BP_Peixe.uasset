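; BP_Peixe is a jumping fish enemy that shuttles along a referenced spline and damages the ThirdPersonCharacter when its mesh overlaps it.
; Two timelines, rate-scaled by TimeToCompleteSeconds, drive location and rotation from spline distance: MovePeixe runs forward and VoltarPeixe runs back with the spline rotation negated.
; Each timeline starts the other after a TimeOfLoop delay, looping endlessly from BeginPlay.
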(event OnComponentBeginOverlap(StaticMesh)
  (params (OverlappedComponent :type Primitive%20Component%20Object%20Reference) (OtherActor :type Actor%20Object%20Reference) (OtherComp :type Primitive%20Component%20Object%20Reference) (OtherBodyIndex :type Integer) (bFromSweep :type Boolean) (SweepResult :type Hit%20Result%20Structure%20%28by%20ref%29))
  (bind _asthird_person_character (Utilities|Casting|CastToThirdPersonCharacter OtherActor))
  (Game|Damage|ApplyDamage _asthird_person_character 1.0 0 0))

(event Custom|MovePeixe
  (bind _splineref (Variables|Default|GetsplineRef))
  (bind _spline (Variables|/Game/Enemys/PeixePulador/BP_SplinePath.BP_SplinePath_C|GetSpline _splineref))
  (Components|Timeline|SetPlayRate (Variables|Default|GetMovePeixeT) (/ 1.0 (Variables|Default|GetTimeToComplete%28Seconds%29)))
  (bind _movetrack (Timeline|MovePeixeT PlayFromStart)
    (:Update
      (Transformation|SetActorLocationAndRotation (Spline|GetLocationatDistanceAlongSpline _spline (Math|Float|Lerp 0.0 (Spline|GetSplineLength (Variables|/Game/Enemys/PeixePulador/BP_SplinePath.BP_SplinePath_C|GetSpline (Variables|Default|GetsplineRef))) _movetrack) "World") (Spline|GetRotationatDistanceAlongSpline _spline (Math|Float|Lerp 0.0 (Spline|GetSplineLength (Variables|/Game/Enemys/PeixePulador/BP_SplinePath.BP_SplinePath_C|GetSpline (Variables|Default|GetsplineRef))) _movetrack) "World")))
    (:Finished
      (Utilities|FlowControl|Delay (Variables|Default|GetTimeOfLoop))
      (CallFunction|VoltarPeixe))))

(event Custom|VoltarPeixe
  (bind _splineref (Variables|Default|GetsplineRef))
  (bind _spline (Variables|/Game/Enemys/PeixePulador/BP_SplinePath.BP_SplinePath_C|GetSpline _splineref))
  (Components|Timeline|SetPlayRate (Variables|Default|GetVoltarPeixeT) (/ 1.0 (Variables|Default|GetTimeToComplete%28Seconds%29)))
  (bind _movetrack (Timeline|VoltarPeixeT PlayFromStart)
    (:Update
      (Transformation|SetActorLocationAndRotation (Spline|GetLocationatDistanceAlongSpline _spline (Math|Float|Lerp (Spline|GetSplineLength (Variables|/Game/Enemys/PeixePulador/BP_SplinePath.BP_SplinePath_C|GetSpline (Variables|Default|GetsplineRef))) 0.0 _movetrack) "World") (* (Spline|GetRotationatDistanceAlongSpline _spline (Math|Float|Lerp (Spline|GetSplineLength (Variables|/Game/Enemys/PeixePulador/BP_SplinePath.BP_SplinePath_C|GetSpline (Variables|Default|GetsplineRef))) 0.0 _movetrack) "World") -1)))
    (:Finished
      (Utilities|FlowControl|Delay (Variables|Default|GetTimeOfLoop))
      (CallFunction|MovePeixe))))

(event EventBeginPlay
  (CallFunction|MovePeixe))

(fn ConstructionScript)