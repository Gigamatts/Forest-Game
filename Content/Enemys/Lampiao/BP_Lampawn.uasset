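; BP_Lampawn is a melee enemy character that senses the player, takes damage and ragdolls on death.
; PawnSensing sets the "HasSeenPlayer?" Blackboard flag, which Tick clears after delays if the player is still within sight radius.
; Non-lethal hits play a reaction montage, launch the Lampawn itself along its forward vector's Y/Z and grant one second of immunity.
; Attack plays a punch montage.
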(event OnSeePawn(PawnSensing)
  (params (Pawn :type Pawn%20Object%20Reference))
  (Utilities|Casting|CastToThirdPersonCharacter Pawn)
  (AI|Components|Blackboard|SetValueasBool (AI|GetBlackboard (AI|GetAIController self)) (Utilities|Name|MakeLiteralName "HasSeenPlayer?") true)
  (Variables|Default|SetcanSeePlayer? true))

(event EventTick
  (params (DeltaSeconds :type Float%20%28single-precision%29))
  (if (Variables|Default|GetcanSeePlayer?)
    (Utilities|FlowControl|Delay 0.5)
    (if (<= (Transformation|GetDistanceTo (Game|Player|GetPlayerPawn 0)) (Variables|/Script/AIModule.PawnSensingComponent|GetSightRadius (Variables|Default|GetPawnSensing)))
      (Utilities|FlowControl|Delay 1.0)
      (Variables|Default|SetcanSeePlayer? false)
      (AI|Components|Blackboard|SetValueasBool (AI|GetBlackboard (AI|GetAIController self)) (Utilities|Name|MakeLiteralName "HasSeenPlayer?") false))))

(event Game|Damage|EventAnyDamage
  (params (Damage :type Float%20%28single-precision%29) (DamageType :type Damage%20Type%20Object%20Reference) (InstigatedBy :type Controller%20Object%20Reference) (DamageCauser :type Actor%20Object%20Reference))
  (bind _returnvalue (Transformation|GetActorForwardVector))
  (bind _charactermovement (Variables|Character|GetCharacterMovement))
  ;[1 0.06146 0.06146] Take Damege
  (if (not (Variables|Default|GetIsImune))
    (bind _output_get (Variables|Default|SetHealth (- (Variables|Default|GetHealth) Damage)))
    (Animation|PlayAnimMontage "/Game/Assets/Models/Lampawn/Animations/LampawnGetHitAnim_Montage.LampawnGetHitAnim_Montage" 1.0 "None")
    (if (<= _output_get 0.0)
      (Collision|SetCollisionResponsetoChannel (Variables|Collision|GetCapsuleComponent) "ECC_Pawn" "ECR_Ignore")
      (Physics|SetSimulatePhysics (Variables|Character|GetMesh) true)
      (else
        ;;[1 1 1] Make player imune and knockback player
        (Variables|Default|SetIsImune true)
        (if (AI|Components|NavMovement|IsFalling _charactermovement)
          (Character|StopJumping)
          (else
            (Variables|/Script/Engine.CharacterMovementComponent|SetGroundFriction _charactermovement 0.0)))
        (Variables|/Script/Engine.MovementComponent|SetVelocity _charactermovement "0, 0, 0")
        (Character|LaunchCharacter (Math|Vector|MakeVector 0.0 (* (.y _returnvalue) 1e+03) (* (.z _returnvalue) 1e+03)) true true)
        ;;[1 1 1] duration imunity of the player
        (Utilities|FlowControl|Delay 1.0)
        (Variables|Default|SetIsImune false)))))

(fn ConstructionScript)

(fn NewFunction0)

(fn Attack
  (bind _returnvalue (Animation|PlayAnimMontage "/Game/Assets/Models/Lampawn/Animations/LampawnPunchAnim_Montage.LampawnPunchAnim_Montage" 1.0 "None"))
  (return _returnvalue))