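; Enemy actor that the player's ThirdPersonCharacter can damage by punching and kill.
; When the character begins overlapping the Capsule while IsPunching is set, Health drops by Damage.
; Tick polls Health and, once it falls below zero, plays a death sound, spawns Enemy_dead_BP at the same transform and destroys the actor.
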(event OnComponentBeginOverlap(Capsule)
  (params (OverlappedComponent :type Primitive%20Component%20Object%20Reference) (OtherActor :type Actor%20Object%20Reference) (OtherComp :type Primitive%20Component%20Object%20Reference) (OtherBodyIndex :type Integer) (bFromSweep :type Boolean) (SweepResult :type Hit%20Result%20Structure%20%28by%20ref%29))
  (bind _asthird_person_character (Utilities|Casting|CastToThirdPersonCharacter OtherActor))
  (if (Variables|/Game/ThirdPersonCPP/Blueprints/ThirdPersonCharacter.ThirdPersonCharacter_C|GetisPunching _asthird_person_character)
    (Variables|Default|SetHealth (- (Variables|Default|GetHealth) (Variables|Default|GetDamage)))))

(event EventBeginPlay)

(event EventTick
  (params (DeltaSeconds :type Float%20%28single-precision%29))
  (if (< (Variables|Default|GetHealth) 0)
    (Audio|PlaySoundatLocation "/Game/Sounds/Death_Cue.Death_Cue" (Transformation|GetActorLocation) "0, 0, 0" 1.0 1.0 0.0 0 0 0)
    (Game|SpawnActorfromClass "/Game/Enemy_dead_BP.Enemy_dead_BP_C" (Transformation|GetActorTransform) "Undefined" 0 0)
    (Actor|DestroyActor)))

(fn ConstructionScript)