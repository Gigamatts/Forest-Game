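; Falling platform prop that drops through physics when triggered by its box overlap, then returns to place.
; When Timed, overlap starts three timeline-driven rotation shakes of rising intensity before the drop; otherwise it drops shortly after the overlap ends.
; After a configurable Time, physics switches off and Tick interpolates the cube's location back to the box position cached at BeginPlay, without resetting rotation.
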(event OnComponentBeginOverlap(Box)
  (params (OverlappedComponent :type Primitive%20Component%20Object%20Reference) (OtherActor :type Actor%20Object%20Reference) (OtherComp :type Primitive%20Component%20Object%20Reference) (OtherBodyIndex :type Integer) (bFromSweep :type Boolean) (SweepResult :type Hit%20Result%20Structure%20%28by%20ref%29))
  (bind _cube (Variables|Default|GetCube))
  ;[1 1 1] Derruba platafora
  (if (Variables|Default|GetTimed?)
    (CallFunction|ShakePlataform)
    (Utilities|FlowControl|Delay 1.0)
    (Variables|Shake|SetShake%20plataform%20Play%20Rate 1.5)
    (Variables|Shake|SetRotationFactor "6.000000, 0, 0")
    (CallFunction|ShakePlataform)
    (Utilities|FlowControl|Delay 1.0)
    (Variables|Shake|SetShake%20plataform%20Play%20Rate 3.0)
    (Variables|Shake|SetRotationFactor "10.000000, 0, 0")
    (CallFunction|ShakePlataform)
    (Utilities|FlowControl|Delay 1.0)
    (Physics|SetSimulatePhysics _cube true)
    (Utilities|FlowControl|Delay (Variables|Default|Gettime))
    (Physics|SetSimulatePhysics _cube false)
    (Variables|Default|SetBackToPlace? true)))

(event OnComponentEndOverlap(Box)
  (params (OverlappedComponent :type Primitive%20Component%20Object%20Reference) (OtherActor :type Actor%20Object%20Reference) (OtherComp :type Primitive%20Component%20Object%20Reference) (OtherBodyIndex :type Integer))
  (bind _cube (Variables|Default|GetCube))
  ;[1 1 1] Derruba platafora
  (if (not (Variables|Default|GetTimed?))
    (Utilities|FlowControl|Delay 0.2)
    (Physics|SetSimulatePhysics _cube true)
    (Utilities|FlowControl|Delay (Variables|Default|Gettime))
    (Physics|SetSimulatePhysics _cube false)
    (Variables|Default|SetBackToPlace? true)))

(event Custom|ShakePlataform
  (Components|Timeline|SetPlayRate (Variables|Default|GetShakePlataformAnim) (Variables|Shake|GetShake%20plataform%20Play%20Rate))
  (bind _alpha (Timeline|ShakePlataformAnim PlayFromStart)
    (:Update
      (Transformation|SetWorldRotation (Variables|Default|GetCube) (Math|Rotator|Lerp(Rotator) (Variables|Shake|GetbaseRotation) (Math|Rotator|CombineRotators (Variables|Shake|GetbaseRotation) (Variables|Shake|GetRotationFactor)) _alpha) false false))))

(event EventBeginPlay
  (Variables|Default|SetOrinalLocation (Transformation|GetWorldLocation (Variables|Default|GetBox))))

(event EventTick
  (params (DeltaSeconds :type Float%20%28single-precision%29))
  (bind _cube (Variables|Default|GetCube))
  ;[1 1 1] Volta a plataforma pro lugar
  (if (Variables|Default|GetBackToPlace?)
    (bind _sweephitresult (Transformation|SetWorldLocation _cube (Math|Interpolation|VInterpTo (Transformation|GetWorldLocation _cube) (Variables|Default|GetOrinalLocation) (Utilities|Time|GetWorldDeltaSeconds) 2.0) false false))
    (if (Math|Vector|Equal(Vector) (.TraceEnd (Collision|BreakHitResult _sweephitresult)) (Variables|Default|GetOrinalLocation) 0.0001)
      (Variables|Default|SetBackToPlace? false))))

(fn ConstructionScript)