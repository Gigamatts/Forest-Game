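; BP_GemFinal is a gem prop that reveals its mesh when the ThirdPersonCharacter first overlaps its box.
; That one-time overlap decrements GemValue on the first HealthBar widget found and sets its GemAlpha to full.
; It then calls CheckGems on the BP_ManagerFinal instance cached at BeginPlay.
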(event OnComponentBeginOverlap(Box)
  (params (OverlappedComponent :type Primitive%20Component%20Object%20Reference) (OtherActor :type Actor%20Object%20Reference) (OtherComp :type Primitive%20Component%20Object%20Reference) (OtherBodyIndex :type Integer) (bFromSweep :type Boolean) (SweepResult :type Hit%20Result%20Structure%20%28by%20ref%29))
  (Utilities|Casting|CastToThirdPersonCharacter OtherActor)
  (Utilities|FlowControl|DoOnce false
    (:Completed
      (Development|SetHiddeninGame (Variables|Default|GetStaticMesh) false false)
      (bind _foundwidgets (Widget|GetAllWidgetsOfClass "/Game/UI/HUD/HealthBar.HealthBar_C" true))
      (Variables|/Game/UI/HUD/HealthBar.HealthBar_C|SetgemValue (Utilities|Array|Get(acopy) _foundwidgets) (- (Variables|/Game/UI/HUD/HealthBar.HealthBar_C|GetgemValue (Utilities|Array|Get(acopy) _foundwidgets)) 1))
      (Variables|/Game/UI/HUD/HealthBar.HealthBar_C|SetgemAlpha (Utilities|Array|Get(acopy) _foundwidgets) 1.0)
      (Default|CheckGems (Variables|Default|GetManagerRef)))))

(event EventBeginPlay
  (bind _outactors (Actor|GetAllActorsOfClass "/Game/Props/Final/BP_ManagerFinal.BP_ManagerFinal_C"))
  (Variables|Default|SetManagerRef (Utilities|Array|Get(acopy) _outactors)))

(fn ConstructionScript)