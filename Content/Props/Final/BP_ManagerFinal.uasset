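; BP_ManagerFinal runs the ending sequence once the player's gem objective is met.
; CheckGems reads GemValue from the first HealthBar widget and, at zero, fires the crystal descent, camera switch and credits events.
; A timeline moves CarrotRef toward a target position while the view blends to this actor with input disabled.
; After a delay, input returns and a TransitionManager widget fades to the configured level.
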(event Custom|CheckGems
  (bind _foundwidgets (Widget|GetAllWidgetsOfClass "/Game/UI/HUD/HealthBar.HealthBar_C" true))
  (if (== (Variables|/Game/UI/HUD/HealthBar.HealthBar_C|GetgemValue (Utilities|Array|Get(acopy) _foundwidgets)) 0)
    (CallFunction|DescerCristal)
    (CallFunction|MudarCamera)
    (CallFunction|ChamarCreditos)))

(event Custom|DescerCristal
  (bind _carrotref (Variables|Default|GetCarrotRef))
  (Rendering|SetActorHiddenInGame (Variables|Default|GetCarrotRef) false)
  (Utilities|FlowControl|Delay 2.5)
  (Components|Timeline|SetPlayRate (Variables|Default|GetDescerCristalAnim) (/ 1.0 (Variables|Default|GetPlayRateSec)))
  (bind _newtrack_0 (Timeline|DescerCristalAnim Play)
    (:Update
      (Transformation|SetActorLocation _carrotref (Math|Vector|Lerp(Vector) (Transformation|GetActorLocation _carrotref) (Variables|Default|GetPosForMove) _newtrack_0) false false))))

(event Custom|MudarCamera
  (bind _playerref (Variables|Default|GetPlayerRef))
  (Input|DisableInput _playerref 0)
  (Variables|/Game/ThirdPersonCPP/Blueprints/ThirdPersonCharacter.ThirdPersonCharacter_C|SetCanRotate _playerref true)
  (Game|Player|SetViewTargetwithBlend (Game|GetPlayerController 0) self 2.0 "VTBlend_Linear" 0.0 false))

(event Custom|ChamarCreditos
  (Utilities|FlowControl|Delay 6.7)
  (Input|EnableInput (Variables|Default|GetPlayerRef) 0)
  (bind _returnvalue (UserInterface|CreateWidget "/Game/UI/TransitionManager.TransitionManager_C" 0 true (Variables|Default|GetlevelToLoad)))
  (UserInterface|Viewport|AddtoViewport _returnvalue 0))

(event EventBeginPlay
  (bind _asthird_person_character (Utilities|Casting|CastToThirdPersonCharacter (Game|GetPlayerCharacter 0)))
  (Variables|Default|SetPlayerRef _asthird_person_character))

(fn ConstructionScript)