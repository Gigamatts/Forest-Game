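; Pushable cube prop that the third-person character can move.
; Two trigger volumes, one for the X axis and one for the Y axis, detect the character on overlap.
; Entering either volume enables physics simulation on the cube and sets the character's IsPushing flag.
; Leaving either volume turns both off again, without checking whether the other volume is still overlapped.
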(event OnComponentEndOverlap(Yaxiscollision)
  (params (OverlappedComponent :type Primitive%20Component%20Object%20Reference) (OtherActor :type Actor%20Object%20Reference) (OtherComp :type Primitive%20Component%20Object%20Reference) (OtherBodyIndex :type Integer))
  ;[1 1 1] Y axxis Collison
  (bind _asthird_person_character (Utilities|Casting|CastToThirdPersonCharacter OtherActor))
  (Physics|SetSimulatePhysics (Variables|Default|GetCube) false)
  (Variables|/Game/ThirdPersonCPP/Blueprints/ThirdPersonCharacter.ThirdPersonCharacter_C|SetisPushing? _asthird_person_character false))

(event OnComponentBeginOverlap(Yaxiscollision)
  (params (OverlappedComponent :type Primitive%20Component%20Object%20Reference) (OtherActor :type Actor%20Object%20Reference) (OtherComp :type Primitive%20Component%20Object%20Reference) (OtherBodyIndex :type Integer) (bFromSweep :type Boolean) (SweepResult :type Hit%20Result%20Structure%20%28by%20ref%29))
  ;[1 1 1] Y axxis Collison
  (bind _asthird_person_character (Utilities|Casting|CastToThirdPersonCharacter OtherActor))
  (Physics|SetSimulatePhysics (Variables|Default|GetCube) true)
  (Variables|/Game/ThirdPersonCPP/Blueprints/ThirdPersonCharacter.ThirdPersonCharacter_C|SetisPushing? _asthird_person_character true))

(event OnComponentBeginOverlap(Xaxiscollision)
  (params (OverlappedComponent :type Primitive%20Component%20Object%20Reference) (OtherActor :type Actor%20Object%20Reference) (OtherComp :type Primitive%20Component%20Object%20Reference) (OtherBodyIndex :type Integer) (bFromSweep :type Boolean) (SweepResult :type Hit%20Result%20Structure%20%28by%20ref%29))
  ;[1 1 1] X axxis Collision
  (bind _asthird_person_character (Utilities|Casting|CastToThirdPersonCharacter OtherActor))
  (Physics|SetSimulatePhysics (Variables|Default|GetCube) true)
  (Variables|/Game/ThirdPersonCPP/Blueprints/ThirdPersonCharacter.ThirdPersonCharacter_C|SetisPushing? _asthird_person_character true))

(event OnComponentEndOverlap(Xaxiscollision)
  (params (OverlappedComponent :type Primitive%20Component%20Object%20Reference) (OtherActor :type Actor%20Object%20Reference) (OtherComp :type Primitive%20Component%20Object%20Reference) (OtherBodyIndex :type Integer))
  ;[1 1 1] X axxis Collision
  (bind _asthird_person_character (Utilities|Casting|CastToThirdPersonCharacter OtherActor))
  (Physics|SetSimulatePhysics (Variables|Default|GetCube) false)
  (Variables|/Game/ThirdPersonCPP/Blueprints/ThirdPersonCharacter.ThirdPersonCharacter_C|SetisPushing? _asthird_person_character false))

(fn ConstructionScript)