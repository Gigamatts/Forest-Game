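; Enemy death prop Blueprint that scatters a set of component pieces, then removes itself.
; On BeginPlay it loops over four components, mostly named as cubes, and applies the same impulse to each along the backward vector.
; After a short delay the actor destroys itself, so the debris is temporary.
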(event EventBeginPlay
  (for _array_element 0
    (Physics|AddImpulse (Utilities|Array|Get(acopy) (Utilities|Array|MakeArray (Variables|Default|GetCube2) (Variables|Default|GetCube1) (Variables|Default|Getw) (Variables|Default|GetCube)) _array_element) (* (Class|KismetMathLibrary|VectorBackward) 1e+02) "None" false))
  (Utilities|FlowControl|Delay 5.0)
  (Actor|DestroyActor))

(fn ConstructionScript)