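; Pressure button prop that toggles a water level actor between its original and raised positions when a ThirdPersonCharacter enters its box.
; Timelines lerp the button down on overlap and back up once the player leaves.
; Each finished press flips SubirDescer on the level's first ManagerAgua, then plays the raise or lower water timeline.
; The lowering branch applies AbaixarAguaPlayRate to SubirAguaAnim, not to the AbaixarAguaAnim it plays.
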(event OnComponentBeginOverlap(StaticMesh1)
  (params (OverlappedComponent :type Primitive%20Component%20Object%20Reference) (OtherActor :type Actor%20Object%20Reference) (OtherComp :type Primitive%20Component%20Object%20Reference) (OtherBodyIndex :type Integer) (bFromSweep :type Boolean) (SweepResult :type Hit%20Result%20Structure%20%28by%20ref%29)))

(event OnComponentEndOverlap(StaticMesh1)
  (params (OverlappedComponent :type Primitive%20Component%20Object%20Reference) (OtherActor :type Actor%20Object%20Reference) (OtherComp :type Primitive%20Component%20Object%20Reference) (OtherBodyIndex :type Integer)))

(event OnComponentBeginOverlap(Box)
  (params (OverlappedComponent :type Primitive%20Component%20Object%20Reference) (OtherActor :type Actor%20Object%20Reference) (OtherComp :type Primitive%20Component%20Object%20Reference) (OtherBodyIndex :type Integer) (bFromSweep :type Boolean) (SweepResult :type Hit%20Result%20Structure%20%28by%20ref%29))
  ;[1 1 1] Begin
  (Utilities|Casting|CastToThirdPersonCharacter OtherActor)
  (if (not (Variables|Default|GetPlayerColidindo))
    (CallFunction|AbaixarBotao)
    (Variables|Default|SetPlayerColidindo true)))

(event OnComponentEndOverlap(Box)
  (params (OverlappedComponent :type Primitive%20Component%20Object%20Reference) (OtherActor :type Actor%20Object%20Reference) (OtherComp :type Primitive%20Component%20Object%20Reference) (OtherBodyIndex :type Integer))
  ;[1 1 1] Begin
  (Utilities|Casting|CastToThirdPersonCharacter OtherActor)
  (Variables|Default|SetPlayerColidindo false)
  (CallFunction|SubirBotao))

(event Custom|AbaixarBotao
  (bind _managerref (Variables|Default|GetManagerRef))
  ;[1 1 1] Abaixar/Subir botão
  (Components|Timeline|SetPlayRate (Variables|Default|GetAbaixarBotaoAnim) (Variables|AnimPlayRate|GetAbaixarBotaoPlayRate))
  (bind _x_location (Timeline|AbaixarBotaoAnim PlayFromStart)
    (:Update
      (Transformation|SetRelativeLocation (Variables|Default|GetStaticMesh1) (Math|Vector|Lerp(Vector) (Variables|/Script/Engine.SceneComponent|GetRelativeLocation (Variables|Default|GetStaticMesh1)) (Variables|Default|GetBotaoPressPosition) _x_location) false false))
    (:Finished
      (Variables|/Game/Props/BotaoSubirAgua/ManagerAgua.ManagerAgua_C|SetSubir/Descer _managerref (not (Variables|/Game/Props/BotaoSubirAgua/ManagerAgua.ManagerAgua_C|GetSubir/Descer _managerref)))
      (CallFunction|SubirAgua)
      (Utilities|FlowControl|Delay 1.0)
      (if (not (Variables|Default|GetPlayerColidindo))
        (CallFunction|SubirBotao)))))

(event Custom|SubirAgua
  ;[1 1 1] Abaixar/Subir
  (if (Variables|/Game/Props/BotaoSubirAgua/ManagerAgua.ManagerAgua_C|GetSubir/Descer (Variables|Default|GetManagerRef))
    (Components|Timeline|SetPlayRate (Variables|Default|GetSubirAguaAnim) (Variables|AnimPlayRate|GetSubirAguaPlayRate))
    (bind _x_location (Timeline|SubirAguaAnim PlayFromStart)
      (:Update
        (Transformation|SetActorLocation (Variables|Default|GetWaterLevel) (Math|Vector|Lerp(Vector) (Variables|Default|GetWaterOriginalPosition_0) (Variables|Default|GetWaterLevelNewPos) _x_location) false false)))
    (else
      (Components|Timeline|SetPlayRate (Variables|Default|GetSubirAguaAnim) (Variables|AnimPlayRate|GetAbaixarAguaPlayRate))
      (bind _x_location_2 (Timeline|AbaixarAguaAnim PlayFromStart)
        (:Update
          (Transformation|SetActorLocation (Variables|Default|GetWaterLevel) (Math|Vector|Lerp(Vector) (Variables|Default|GetWaterLevelNewPos) (Variables|Default|GetWaterOriginalPosition_0) _x_location_2) false false))))))

(event Custom|SubirBotao
  ;[1 1 1] Abaixar/Subir botão
  (bind _x_location (Timeline|SubirBotaoAnim Play)
    (:Update
      (Transformation|SetRelativeLocation (Variables|Default|GetStaticMesh1) (Math|Vector|Lerp(Vector) (Variables|/Script/Engine.SceneComponent|GetRelativeLocation (Variables|Default|GetStaticMesh1)) (Variables|Default|GetBotaoOriginalPosition) _x_location) false false))))

(event EventBeginPlay
  ;[1 1 1] Begin
  (Variables|Default|SetBotaoOriginalPosition (Variables|/Script/Engine.SceneComponent|GetRelativeLocation (Variables|Default|GetStaticMesh1)))
  (Variables|Default|SetWaterOriginalPosition_0 (Transformation|GetActorLocation (Variables|Default|GetWaterLevel)))
  (bind _outactors (Actor|GetAllActorsOfClass "/Game/Props/BotaoSubirAgua/ManagerAgua.ManagerAgua_C"))
  (bind _asmanager_agua (Utilities|Casting|CastToManagerAgua (Utilities|Array|Get(acopy) _outactors)))
  (Variables|Default|SetManagerRef _asmanager_agua))

(fn ConstructionScript)