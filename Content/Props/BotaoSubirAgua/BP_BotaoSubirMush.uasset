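; One-shot floor button that moves two mushroom actors when the player character steps on it.
; Overlap destroys the trigger box, sets PodeAbaixar and plays a press timeline, which then chains timelines lerping MushroomPraDescer and then MushroomPraSubir to target positions.
; On BeginPlay, PodeAbaixarSaved from the "save1" slot replays the mushroom movement without a press; this Blueprint never writes the save.
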(event OnComponentBeginOverlap(Box)
  (params (OverlappedComponent :type Primitive%20Component%20Object%20Reference) (OtherActor :type Actor%20Object%20Reference) (OtherComp :type Primitive%20Component%20Object%20Reference) (OtherBodyIndex :type Integer) (bFromSweep :type Boolean) (SweepResult :type Hit%20Result%20Structure%20%28by%20ref%29))
  ;[1 1 1] Begin
  (Utilities|Casting|CastToThirdPersonCharacter OtherActor)
  (CallFunction|AbaixarBotao)
  (Components|DestroyComponent (Variables|Default|GetBox))
  (Variables|Default|SetPodeAbaixar true))

(event Custom|AbaixarBotao
  ;[1 1 1] Abaixar/Subir botão
  (Components|Timeline|SetPlayRate (Variables|Default|GetAbaixarBotaoAnim) (Variables|AnimPlayRate|GetAbaixarBotaoPlayRate))
  (bind _x_location (Timeline|AbaixarBotaoAnim PlayFromStart)
    (:Update
      (Transformation|SetRelativeLocation (Variables|Default|GetStaticMesh1) (Math|Vector|Lerp(Vector) (Variables|/Script/Engine.SceneComponent|GetRelativeLocation (Variables|Default|GetStaticMesh1)) (Variables|Default|GetBotaoPressPosition) _x_location) false false))
    (:Finished
      (CallFunction|SubirCogumelo))))

(event Custom|SubirCogumelo
  (bind _mushroompradescer (Variables|Default|GetMushroomPraDescer))
  (bind _mushroomprasubir (Variables|Default|GetMushroomPraSubir))
  ;[1 1 1] Abaixar/Subir
  (Components|Timeline|SetPlayRate (Variables|Default|GetSubirAguaAnim) (Variables|AnimPlayRate|GetSubirAguaPlayRate))
  (bind _x_location (Timeline|SubirAguaAnim PlayFromStart)
    (:Update
      (Transformation|SetActorLocation _mushroompradescer (Math|Vector|Lerp(Vector) (Transformation|GetActorLocation _mushroompradescer) (Variables|Default|GetMushroomDescer) _x_location) false false))
    (:Finished
      (Components|Timeline|SetPlayRate (Variables|Default|GetSubirAguaAnim) (Variables|AnimPlayRate|GetAbaixarAguaPlayRate))
      (bind _x_location_2 (Timeline|AbaixarAguaAnim PlayFromStart)
        (:Update
          (Transformation|SetActorLocation _mushroomprasubir (Math|Vector|Lerp(Vector) (Transformation|GetActorLocation _mushroomprasubir) (Variables|Default|GetMushroomSubir) _x_location_2) false false))))))

(event EventBeginPlay
  (bind _returnvalue (SaveGame|LoadGamefromSlot "save1"))
  (bind _asbp_save_game (Utilities|Casting|CastToBP_SaveGame _returnvalue))
  (if (Variables|/Game/Props/BP_SaveGame.BP_SaveGame_C|GetPodeAbaixarSaved _asbp_save_game)
    (CallFunction|SubirCogumelo)
    (Development|PrintString "Chamou")))

(fn ConstructionScript)