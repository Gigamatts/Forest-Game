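; Checkpoint prop that saves the game when the player character overlaps its box and shows a flower while it is active.
; The overlap records itself as CheckpointUsed in slot "save1", calls the GameMode's SaveGame, and plays a timeline that scales the flower up once per activation.
; AttCheckPoint re-runs itself each second, reloading the save to show the flower or hide and reset it when another checkpoint is current.
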(event OnComponentBeginOverlap(Box)
  (params (OverlappedComponent :type Primitive%20Component%20Object%20Reference) (OtherActor :type Actor%20Object%20Reference) (OtherComp :type Primitive%20Component%20Object%20Reference) (OtherBodyIndex :type Integer) (bFromSweep :type Boolean) (SweepResult :type Hit%20Result%20Structure%20%28by%20ref%29))
  ;[1 1 1] Salvar pos
  (Utilities|Casting|CastToThirdPersonCharacter OtherActor)
  (bind _returnvalue (SaveGame|LoadGamefromSlot "save1"))
  (bind _asbp_save_game (Utilities|Casting|CastToBP_SaveGame _returnvalue))
  (Variables|/Game/Props/BP_SaveGame.BP_SaveGame_C|SetCheckpointUsed _asbp_save_game self)
  (SaveGame|SaveGametoSlot _asbp_save_game "save1")
  (bind _asbp_game_mode (Utilities|Casting|CastToBP_GameMode (Game|GetGameMode)))
  (Default|SaveGame _asbp_game_mode)
  (CallFunction|AttCheckPoint)
  (if (not (Variables|Default|GetJaFoiPego))
    (CallFunction|FlowerGrow)))

(event Custom|AttCheckPoint
  ;[1 1 1] Checar se ta ativo ou n
  (bind _returnvalue (SaveGame|LoadGamefromSlot "save1"))
  (bind _asbp_save_game (Utilities|Casting|CastToBP_SaveGame _returnvalue))
  (if (== (Variables|/Game/Props/BP_SaveGame.BP_SaveGame_C|GetCheckpointUsed _asbp_save_game) self)
    (Development|SetHiddeninGame (Variables|Default|GetFlower) false true)
    (Utilities|FlowControl|Delay 1.0)
    (CallFunction|AttCheckPoint)
    (else
      (Development|SetHiddeninGame (Variables|Default|GetFlower) true true)
      (Transformation|SetRelativeScale3D (Variables|Default|GetFlower) "0, 0, 0")
      (Variables|Default|SetJaFoiPego false)
      (Utilities|FlowControl|Delay 1.0)
      (CallFunction|AttCheckPoint))))

(event Custom|FlowerGrow
  ;[1 1 1] Animação de coleta
  (Variables|Default|SetJaFoiPego true)
  (Components|Timeline|SetPlayRate (Variables|Default|GetFlowerGrowAnim) (/ 1.0 (Variables|Default|GetTimeToComplete)))
  (bind _newtrack_0 (Timeline|FlowerGrowAnim PlayFromStart)
    (:Update
      (Transformation|SetRelativeScale3D (Variables|Default|GetFlower) (Math|Vector|Lerp(Vector) (Variables|Default|GetBaseScale) (Variables|Default|GetNewScale) _newtrack_0)))))

(event EventBeginPlay
  (Variables|Default|SetBaseScale (Variables|/Script/Engine.SceneComponent|GetRelativeScale3D (Variables|Default|GetFlower)))
  (CallFunction|AttCheckPoint))

(fn ConstructionScript)