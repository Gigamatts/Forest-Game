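; BP_Door is a door prop, filed under a door-with-button folder, that slides down along its local Z axis when OpenDoor is called.
; OpenDoor plays the SubirAnim timeline at the inverse of NewPlayRate.
; Each update lerps the static mesh from its current relative location toward a point slightly lower, so movement accumulates per tick rather than following fixed endpoints.
; The file has no closing logic.
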(event Custom|OpenDoor
  (bind _staticmesh (Variables|Default|GetStaticMesh))
  (bind _relativelocation (Variables|/Script/Engine.SceneComponent|GetRelativeLocation _staticmesh))
  (Components|Timeline|SetPlayRate (Variables|Default|GetSubirAnim) (/ 1.0 (Variables|Default|GetNewPlayRate)))
  (bind _newtrack_0 (Timeline|SubirAnim Play)
    (:Update
      (Transformation|SetRelativeLocation _staticmesh (Math|Vector|Lerp(Vector) (Variables|/Script/Engine.SceneComponent|GetRelativeLocation _staticmesh) (Math|Vector|MakeVector (.x _relativelocation) (.y _relativelocation) (- (.z _relativelocation) 1e+01)) _newtrack_0) false false))))

(fn ConstructionScript)