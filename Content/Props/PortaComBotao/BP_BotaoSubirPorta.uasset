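; A one-shot floor-style button that opens a linked door when a ThirdPersonCharacter overlaps its trigger box.
; The first valid overlap calls OpenDoor on DoorRef, starts the press, destroys the box and plays a bonus sound.
; The press uses a timeline with adjustable play rate to lerp the button mesh from its current relative location toward a pressed position.
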(event OnComponentBeginOverlap(Box)
  (params (OverlappedComponent :type Primitive%20Component%20Object%20Reference) (OtherActor :type Actor%20Object%20Reference) (OtherComp :type Primitive%20Component%20Object%20Reference) (OtherBodyIndex :type Integer) (bFromSweep :type Boolean) (SweepResult :type Hit%20Result%20Structure%20%28by%20ref%29))
  ;[1 1 1] Begin
  (Utilities|Casting|CastToThirdPersonCharacter OtherActor)
  (Utilities|FlowControl|DoOnce false
    (:Completed
      (Default|OpenDoor (Variables|Default|GetDoorRef))
      (CallFunction|AbaixarBotao)
      (Components|DestroyComponent (Variables|Default|GetBox))
      (Audio|PlaySoundatLocation "/Game/Assets/Sounds/bonus-143026_Cue.bonus-143026_Cue" (Transformation|GetActorLocation) "0, 0, 0" 1.0 1.0 0.0 0 0 0))))

(event Custom|AbaixarBotao
  ;[1 1 1] Abaixar/Subir botão
  (Components|Timeline|SetPlayRate (Variables|Default|GetAbaixarBotaoAnim) (Variables|AnimPlayRate|GetAbaixarBotaoPlayRate))
  (bind _x_location (Timeline|AbaixarBotaoAnim PlayFromStart)
    (:Update
      (Transformation|SetRelativeLocation (Variables|Default|GetStaticMesh1) (Math|Vector|Lerp(Vector) (Variables|/Script/Engine.SceneComponent|GetRelativeLocation (Variables|Default|GetStaticMesh1)) (Variables|Default|GetBotaoPressPosition) _x_location) false false))))

(fn ConstructionScript)