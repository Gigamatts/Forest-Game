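; Game mode that manages checkpoint saving, loading, restarting and level transitions through a single BP_SaveGame slot.
; BeginPlay creates the save or restores the player's transform, health and camera; the water manager (ManagerAgua) state returns only without a saved location.
; Separate events store position and status (health, gems, camera, inverted water state).
; Load restarts the level so BeginPlay reapplies data; restart deletes the slot; level change clears save flags and shows a LevelLabel widget.
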(event Custom|Save%20Game
  ;[1 1 1] Save Game
  (bind _returnvalue (SaveGame|LoadGamefromSlot "save1"))
  (bind _asbp_save_game (Utilities|Casting|CastToBP_SaveGame _returnvalue))
  (Variables|/Game/Props/BP_SaveGame.BP_SaveGame_C|SetCharTransform _asbp_save_game (Transformation|GetActorTransform (.AsThird%20Person%20Character (Utilities|Casting|CastToThirdPersonCharacter (Game|GetPlayerCharacter 0)))))
  (Variables|/Game/Props/BP_SaveGame.BP_SaveGame_C|SetUsedSaveLocation _asbp_save_game true)
  (SaveGame|SaveGametoSlot _asbp_save_game "save1"))

(event Custom|Load%20Game
  ;[1 1 1] Load Game
  (Development|ExecuteConsoleCommand "RestartLevel" 0))

(event Custom|Restart%20Game
  ;[1 1 1] Restart/ Delete
  (SaveGame|DeleteGameinSlot "save1")
  (Development|ExecuteConsoleCommand "RestartLevel" 0))

(event Custom|ChangeLevels
  (params (levelName :type Name))
  ;[1 1 1] Change levels
  (bind _returnvalue (SaveGame|LoadGamefromSlot "save1"))
  (bind _asbp_save_game (Utilities|Casting|CastToBP_SaveGame _returnvalue))
  (Variables|/Game/Props/BP_SaveGame.BP_SaveGame_C|SetUsedSaveLocation _asbp_save_game false)
  (Variables|/Game/Props/BP_SaveGame.BP_SaveGame_C|SetUsedSaveLife _asbp_save_game false)
  (Variables|/Game/Props/BP_SaveGame.BP_SaveGame_C|SetGemTableSaved _asbp_save_game (Utilities|Array|MakeArray false false false false false))
  (SaveGame|SaveGametoSlot _asbp_save_game "save1")
  (bind _returnvalue_2 (UserInterface|CreateWidget "/Game/UI/LevelLabel.LevelLabel_C" 0 levelName))
  (UserInterface|Viewport|AddtoViewport _returnvalue_2 0))

(event Custom|SaveStatus
  (bind _returnvalue (Game|GetPlayerCharacter 0))
  (bind _asthird_person_character (Utilities|Casting|CastToThirdPersonCharacter _returnvalue))
  (bind _hudwidget (Variables|/Game/ThirdPersonCPP/Blueprints/ThirdPersonCharacter.ThirdPersonCharacter_C|GetHUDWidget _asthird_person_character))
  ;[1 1 1] Save Status Player Value
  (bind _returnvalue_2 (SaveGame|LoadGamefromSlot "save1"))
  (bind _asbp_save_game (Utilities|Casting|CastToBP_SaveGame _returnvalue_2))
  (Variables|/Game/Props/BP_SaveGame.BP_SaveGame_C|SetLife_Player _asbp_save_game (Variables|/Game/UI/HUD/HealthBar.HealthBar_C|GethealthValue _hudwidget))
  (Variables|/Game/Props/BP_SaveGame.BP_SaveGame_C|SetGemAmount _asbp_save_game (Variables|/Game/UI/HUD/HealthBar.HealthBar_C|GetgemValue _hudwidget))
  (bind _outactors (Actor|GetAllActorsOfClass "/Game/Props/GemManager.GemManager_C"))
  (Variables|/Game/Props/BP_SaveGame.BP_SaveGame_C|SetGemTableSaved _asbp_save_game (Variables|/Game/Props/GemManager.GemManager_C|GetgemTable (Utilities|Array|Get(acopy) _outactors)))
  (Variables|/Game/Props/BP_SaveGame.BP_SaveGame_C|SetUsedSaveLife _asbp_save_game true)
  (Variables|/Game/Props/BP_SaveGame.BP_SaveGame_C|SetUsedJustRotateCamera _asbp_save_game (Variables|/Game/ThirdPersonCPP/Blueprints/ThirdPersonCharacter.ThirdPersonCharacter_C|GetJust%20Rotate%20Camera _asthird_person_character))
  (Variables|/Game/Props/BP_SaveGame.BP_SaveGame_C|SetUsedBoomLocation _asbp_save_game (Variables|/Game/ThirdPersonCPP/Blueprints/ThirdPersonCharacter.ThirdPersonCharacter_C|GetBoomRotation _asthird_person_character))
  (bind _outactors_2 (Actor|GetAllActorsOfClass "/Game/Props/BotaoSubirAgua/ManagerAgua.ManagerAgua_C"))
  (Variables|/Game/Props/BP_SaveGame.BP_SaveGame_C|SetPodeAbaixarSaved _asbp_save_game (not (Variables|/Game/Props/BotaoSubirAgua/ManagerAgua.ManagerAgua_C|GetSubir/Descer (Utilities|Array|Get(acopy) _outactors_2))))
  (SaveGame|SaveGametoSlot _asbp_save_game "save1"))

(event EventBeginPlay
  (bind _returnvalue (SaveGame|DoesSaveGameExist "save1"))
  (if _returnvalue
    (bind _returnvalue_2 (SaveGame|LoadGamefromSlot "save1"))
    (bind _asbp_save_game (Utilities|Casting|CastToBP_SaveGame _returnvalue_2))
    (if (Variables|/Game/Props/BP_SaveGame.BP_SaveGame_C|GetUsedSaveLocation _asbp_save_game)
      ;[1 1 1] load Game functionality
      (bind _asthird_person_character (Utilities|Casting|CastToThirdPersonCharacter (Game|GetPlayerCharacter 0)))
      (Transformation|SetWorldTransform (Variables|/Script/Engine.Character|GetCapsuleComponent _asthird_person_character) (Variables|/Game/Props/BP_SaveGame.BP_SaveGame_C|GetCharTransform _asbp_save_game) false false)
      (Utilities|FlowControl|Delay 0.2)
      (Default|HealthSave _asthird_person_character)
      (Default|SetSavedCameraPos _asthird_person_character)
      (elif (Variables|/Game/Props/BP_SaveGame.BP_SaveGame_C|GetUsedSaveLife _asbp_save_game)
        (bind _asthird_person_character_2 (Utilities|Casting|CastToThirdPersonCharacter (Game|GetPlayerCharacter 0)))
        (Utilities|FlowControl|Delay 0.2)
        (Default|HealthSave _asthird_person_character_2)
        (Default|SetSavedCameraPos _asthird_person_character_2)
        (bind _outactors (Actor|GetAllActorsOfClass "/Game/Props/BotaoSubirAgua/ManagerAgua.ManagerAgua_C"))
        (Variables|/Game/Props/BotaoSubirAgua/ManagerAgua.ManagerAgua_C|SetSubir/Descer (Utilities|Array|Get(acopy) _outactors) (Variables|/Game/Props/BP_SaveGame.BP_SaveGame_C|GetPodeAbaixarSaved _asbp_save_game))))
    (else
      ;[1 1 1] Create Save File
      (bind _returnvalue_3 (SaveGame|CreateSaveGameObject "/Game/Props/BP_SaveGame.BP_SaveGame_C"))
      (SaveGame|SaveGametoSlot _returnvalue_3 "save1"))))

(fn ConstructionScript)